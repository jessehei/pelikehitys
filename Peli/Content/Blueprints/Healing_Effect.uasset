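; Healing effect Blueprint that changes a player character's LifeForce when its ApplyEffect event runs.
; If LifeForce is below the hardcoded maximum of 100, it is set to the Heal value, replacing rather than adding, or to 100 when the sum would exceed that.
; The same branch then sets the effect's own Speed variable to a fixed value.
; BeginPlay, overlap and Tick events are disabled stubs.
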(event EventBeginPlay
  (|CallParentFunction) ; This node is disabled and will not be called.\nDrag off pins to build functionality.
)

(event Collision|EventActorBeginOverlap
  (params (OtherActor :type Actor%20Object%20Reference))
  (|CallParentFunction OtherActor) ; This node is disabled and will not be called.\nDrag off pins to build functionality.
)

(event EventTick
  (params (DeltaSeconds :type Float%20%28single-precision%29))
  (|CallParentFunction DeltaSeconds) ; This node is disabled and will not be called.\nDrag off pins to build functionality.
)

(event EventApplyEffect
  (params (Player%20Character :type Game%20Character%20Object%20Reference))
  (bind _heal (Variables|Default|GetHeal))
  ;[1 1 1] Is lifeforce already max
  (if (< (Variables|/Game/Blueprints/Game_Character.Game_Character_C|GetlifeForce Player%20Character) 1e+02)
    ;[1 1 1] Last calculations for healing
    (if (<= (+ (Variables|/Game/Blueprints/Game_Character.Game_Character_C|GetlifeForce Player%20Character) _heal) 1e+02)
      (Variables|/Game/Blueprints/Game_Character.Game_Character_C|SetlifeForce Player%20Character _heal)
      (else
        (Variables|/Game/Blueprints/Game_Character.Game_Character_C|SetlifeForce Player%20Character 1e+02)))
    (Variables|Default|SetSpeed 7e+02)))

(fn ConstructionScript
  (|CallParentFunction))