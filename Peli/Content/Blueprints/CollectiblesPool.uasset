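; CollectiblesPool is an object pool actor for collectibles in a side-scrolling game.
; CreateCollectible spawns a collectible at the right edge with random height and speed, adding it to the pool until the maximum count is reached.
; UpdateCollectibles moves each one left by its speed and recycles any past the left edge to the right with new random height and speed.
; Its own event graph is empty, so both functions rely on external calls.
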(event EventBeginPlay)

(event Collision|EventActorBeginOverlap
  (params (OtherActor :type Actor%20Object%20Reference)))

(event EventTick
  (params (DeltaSeconds :type Float%20%28single-precision%29)))

(fn ConstructionScript)

(fn CreateCollectible
  ;[1 1 1] Create collectibles if less than max number
  (if (< (Variables|Default|GetnumofCollectibles) (Variables|Default|GetmaxNumofCollectibles))
    ;[1 1 1] Create collectible
    (bind _returnvalue (Game|SpawnActorfromClass "/Game/Blueprints/Collectible.Collectible_C" (Math|Transform|MakeTransform (Math|Vector|MakeVector (Variables|Default|GetcollectibleStartLoc) 0.0 (Math|Random|RandomFloatinRange -5e+02 7e+02))) "Undefined" 0 0))
    (Variables|/Game/Blueprints/Collectible.Collectible_C|SetSpeed _returnvalue (Math|Random|RandomFloatinRange 0.5 (Variables|/Game/Blueprints/Collectible.Collectible_C|GetSpeed _returnvalue)))
    ;[1 1 1] Add collectible to pool
    (Utilities|Array|Insert (Variables|Default|GetthePool) _returnvalue (Variables|Default|GetnumofCollectibles))
    (Math|Integer|IncrementInt (Variables|Default|GetnumofCollectibles))))

(fn UpdateCollectibles
  ;[1 1 1] Update each collectible in pool
  (for _array_element (Variables|Default|GetthePool)
    ;[1 1 1] Check if collectible is out of screen
    (LocalVariables|SetarrayElement _array_element)
    (if (< (.X (Math|Vector|BreakVector (Transformation|GetWorldLocation (Variables|/Script/Engine.Actor|GetRootComponent _array_element)))) (- 0.0 (Variables|Default|GetcollectibleStartLoc)))
      ;[1 1 1] Move collecible to right side of screen
      (Transformation|SetWorldLocation (Variables|/Script/Engine.Actor|GetRootComponent (LocalVariables|GetarrayElement)) (Math|Vector|MakeVector (Variables|Default|GetcollectibleStartLoc) 0.0 (Math|Random|RandomFloatinRange -5e+02 7e+02)) false false)
      (bind _ascollectible (Utilities|Casting|CastToCollectible (LocalVariables|GetarrayElement)))
      (Variables|/Game/Blueprints/Collectible.Collectible_C|SetSpeed _ascollectible (Math|Random|RandomFloatinRange 5.0 25.0))
      (else
        ;[1 1 1] Move collectible
        (bind _ascollectible_2 (Utilities|Casting|CastToCollectible _array_element))
        (Transformation|AddWorldOffset (Variables|/Script/Engine.Actor|GetRootComponent _array_element) (Math|Vector|MakeVector (- 0.0 (Variables|/Game/Blueprints/Collectible.Collectible_C|GetSpeed _ascollectible_2)) 0.0 0.0) false false)))))