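; Paper2D player character that moves along the world X axis and jumps, switching flipbook animations.
; Forward and backward axis inputs shift the capsule by a fixed step per update, without sweep or delta-time scaling.
; Jump sets the idle flipbook and an airborne flag.
; A capsule hit on an object named "Floor" restores the run flipbook and clears the flag.
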(event OnComponentHit(CapsuleComponent)
  (params (HitComponent :type Primitive%20Component%20Object%20Reference) (OtherActor :type Actor%20Object%20Reference) (OtherComp :type Primitive%20Component%20Object%20Reference) (NormalImpulse :type Vector :default "0, 0, 0") (Hit :type Hit%20Result%20Structure%20%28by%20ref%29))
  ;[1 1 1] Stop Jump
  (if (Utilities|Enum|Equal(Enum) (Utilities|GetObjectName OtherActor) "Floor")
    (Sprite|SetFlipbook (Variables|Default|GetSprite) "/Game/Flipbooks/RunAnim.RunAnim")
    (Variables|Default|SetisAirborne false)))

(event EventBeginPlay)

(event Collision|EventActorBeginOverlap
  (params (OtherActor :type Actor%20Object%20Reference)))

(event EventTick
  (params (DeltaSeconds :type Float%20%28single-precision%29)))

(event Input|ActionEvents|InputActionJump
  (params (Key :type Key%20Structure))
  ;[1 1 1] Start Jump
  (:Pressed
    (Character|Jump)
    (Sprite|SetFlipbook (Variables|Default|GetSprite) "/Game/Flipbooks/IdleAnim.IdleAnim")
    (Variables|Default|SetisAirborne true)))

(event Input|AxisEvents|InputAxisMove_Fwd
  (params (AxisValue :type Float%20%28single-precision%29))
  (bind _capsulecomponent (Variables|Collision|GetCapsuleComponent))
  (bind _returnvalue (Transformation|GetWorldLocation _capsulecomponent))
  (bind (_x _y _z) (Math|Vector|BreakVector _returnvalue))
  ;[1 1 1] Move Forward
  (if (> AxisValue 0.0)
    (Transformation|SetWorldLocation _capsulecomponent (Math|Vector|MakeVector (+ _x 1e+01) _y _z) false false)))

(event Input|AxisEvents|InputAxisMove_Bck
  (params (AxisValue :type Float%20%28single-precision%29))
  (bind _capsulecomponent (Variables|Collision|GetCapsuleComponent))
  (bind _returnvalue (Transformation|GetWorldLocation _capsulecomponent))
  (bind (_x _y _z) (Math|Vector|BreakVector _returnvalue))
  ;[1 1 1] Move Backward
  (if (> AxisValue 0.0)
    (Transformation|SetWorldLocation _capsulecomponent (Math|Vector|MakeVector (+ _x -1e+01) _y _z) false false)))

(fn ConstructionScript)