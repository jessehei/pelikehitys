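; Damage effect Blueprint that reduces a player character's LifeForce when its ApplyEffect event fires.
; ApplyEffect subtracts Damage from LifeForce, setting it to zero if the result would be negative, then sets its Speed to 700.
; All other event nodes are disabled, and the construction script only calls its parent.
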(event EventBeginPlay
  (|CallParentFunction) ; This node is disabled and will not be called.\nDrag off pins to build functionality.
)

(event Collision|EventActorBeginOverlap
  (params (OtherActor :type Actor%20Object%20Reference))
  (|CallParentFunction OtherActor) ; This node is disabled and will not be called.\nDrag off pins to build functionality.
)

(event EventTick
  (params (DeltaSeconds :type Float%20%28single-precision%29))
  (|CallParentFunction DeltaSeconds) ; This node is disabled and will not be called.\nDrag off pins to build functionality.
)

(event EventApplyEffect
  (params (Player%20Character :type Game%20Character%20Object%20Reference))
  ;[1 1 1] Last calculations for damage
  (if (>= (- (Variables|/Game/Blueprints/Game_Character.Game_Character_C|GetlifeForce Player%20Character) (Variables|Default|GetDamage)) 0.0)
    (Variables|/Game/Blueprints/Game_Character.Game_Character_C|SetlifeForce Player%20Character (- (Variables|/Game/Blueprints/Game_Character.Game_Character_C|GetlifeForce Player%20Character) (Variables|Default|GetDamage)))
    (else
      (Variables|/Game/Blueprints/Game_Character.Game_Character_C|SetlifeForce Player%20Character 0.0)))
  (Variables|Default|SetSpeed 7e+02))

(fn ConstructionScript
  (|CallParentFunction))